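; BP_SpeedUpPanel is a pinball boost panel that speeds up a ball entering its box trigger and awards score.
; A timeline lerps the root from its starting transform by configurable location and rotation offsets, with a FlipFlop alternating reverse and play for endless back-and-forth motion.
; On overlap with BP_Pinball, it applies an impulse scaled from the ball's velocity, plays a whoosh sound and reports points to BP_FirstPersonGameMode.
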(event OnComponentBeginOverlap(Box)
  (params (OverlappedComponent :type Primitive%20Component%20Object%20Reference) (OtherActor :type Actor%20Object%20Reference) (OtherComp :type Primitive%20Component%20Object%20Reference) (OtherBodyIndex :type Integer) (bFromSweep :type Boolean) (SweepResult :type Hit%20Result%20Structure%20%28by%20ref%29))
  (bind _returnvalue (Transformation|GetActorLocation OtherActor))
  (Utilities|Casting|CastToBP_Pinball OtherActor)
  (Physics|AddImpulseatLocation OtherComp (* (Transformation|GetVelocity OtherActor) (* (Variables|Default|GetSpeedUpPower) 1e+02)) _returnvalue "None")
  (Audio|PlaySoundatLocation "/Game/Sound_PinBall/パンチの風切り音（スローモーション）2.パンチの風切り音（スローモーション）2" _returnvalue "0, 0, 0" 1.0 1.0 0.0 0 0 0 0)
  (bind _asbp_first_person_game_mode (Utilities|Casting|CastToBP_FirstPersonGameMode (Game|GetGameMode)))
  (Default|EventAddScore _asbp_first_person_game_mode (Variables|Default|GetAddScore)))

(event EventBeginPlay
  ;[1 1 1] 往復移動＆回転ループ
  (Variables|Default|SetStartLocation (Transformation|GetWorldLocation (Variables|Default|GetDefaultSceneRoot)))
  (Variables|Default|SetStartRotation (Transformation|GetWorldRotation (Variables|Default|GetDefaultSceneRoot)))
  (bind _alpha (Timeline|タイムライン Play)
    (:Update
      (Transformation|SetWorldLocationAndRotation (Variables|Default|GetDefaultSceneRoot) (Math|Vector|Lerp(Vector) (Variables|Default|GetStartLocation) (+ (Variables|Default|GetStartLocation) (Variables|Default|GetEndLocation)) (* _alpha 2.0)) (Math|Rotator|Lerp(Rotator) (Variables|Default|GetStartRotation) (Math|Rotator|CombineRotators (Variables|Default|GetStartRotation) (Variables|Default|GetEndRotation)) (* _alpha 2.0) true) false false))
    (:Finished
      (Utilities|FlowControl|FlipFlop
        (:A
          (Timeline|タイムライン Reverse))
        (:B
          (Timeline|タイムライン Play))))))

(fn ConstructionScript)