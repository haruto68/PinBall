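; BP_Numbers is a pachinko-style digit actor for the pinball game that displays one of eight number meshes, 0 to 7.
; BeginPlay sets the initial mesh, scale and yaw, then hides the mesh; nothing here re-shows it.
; The placeholder event kari advances Number with wraparound, swaps the mesh through SetMeshNumber, and starts two timelines that animate a yaw spin and a scale effect.
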(event Custom|Anime%20Rotation
  (bind _staticmesh (Variables|Default|GetStaticMesh))
  (bind _returnvalue (Transformation|GetWorldRotation _staticmesh))
  ;[1 1 1] 回転アニメ
  (bind _alpha (Timeline|RotateTimeline PlayFromStart)
    (:Update
      (Transformation|SetRelativeRotation _staticmesh (Math|Rotator|MakeRotator (.roll _returnvalue) (.pitch _returnvalue) (Math|Float|Lerp -2.7e+02 9e+01 _alpha)) false false))))

(event Custom|kari
  (if (< (Variables|Default|GetNumber) 7)
    (Variables|Default|SetNumber (+ (Variables|Default|GetNumber) 1))
    (else
      (Variables|Default|SetNumber 0)))
  (CallFunction|SetMeshNumber (Variables|Default|GetNumber))
  (CallFunction|AnimeScale)
  (CallFunction|AnimeRotation))

(event Custom|Anime%20Scale
  ;[1 1 1] 拡大アニメ
  (bind _alpha (Timeline|Scale%20Timeline PlayFromStart)
    (:Update
      (Transformation|SetRelativeScale3D (Variables|Default|GetStaticMesh) (Math|Conversions|ToVector(Float) (* _alpha (Variables|Default|GetScale)))))))

(event EventBeginPlay
  (CallFunction|SetMeshNumber (Variables|Default|GetNumber))
  (Transformation|SetRelativeScale3D (Variables|Default|GetStaticMesh) (Math|Conversions|ToVector(Float) (Variables|Default|GetScale)))
  (Transformation|SetRelativeRotation (Variables|Default|GetStaticMesh) (Math|Rotator|MakeRotator 0.0 0.0 9e+01) false false)
  (Rendering|SetVisibility (Variables|Default|GetStaticMesh) false false))

(event Collision|EventActorBeginOverlap
  (params (OtherActor :type Actor%20Object%20Reference)))

(event EventTick
  (params (DeltaSeconds :type Float%20%28single-precision%29)))

(fn ConstructionScript)

(fn SetMeshNumber
  (params (num :type Integer))
  (switch int num
    (:0
      (Components|StaticMesh|SetStaticMesh (Variables|Default|GetStaticMesh) "/Game/UMG/Number_3D/Pachinko_number_0.Pachinko_number_0"))
    (:1
      (Components|StaticMesh|SetStaticMesh (Variables|Default|GetStaticMesh) "/Game/UMG/Number_3D/Pachinko_number_1.Pachinko_number_1"))
    (:2
      (Components|StaticMesh|SetStaticMesh (Variables|Default|GetStaticMesh) "/Game/UMG/Number_3D/Pachinko_number_2.Pachinko_number_2"))
    (:3
      (Components|StaticMesh|SetStaticMesh (Variables|Default|GetStaticMesh) "/Game/UMG/Number_3D/Pachinko_number_3.Pachinko_number_3"))
    (:4
      (Components|StaticMesh|SetStaticMesh (Variables|Default|GetStaticMesh) "/Game/UMG/Number_3D/Pachinko_number_4.Pachinko_number_4"))
    (:5
      (Components|StaticMesh|SetStaticMesh (Variables|Default|GetStaticMesh) "/Game/UMG/Number_3D/Pachinko_number_5.Pachinko_number_5"))
    (:6
      (Components|StaticMesh|SetStaticMesh (Variables|Default|GetStaticMesh) "/Game/UMG/Number_3D/Pachinko_number_6.Pachinko_number_6"))
    (:7
      (Components|StaticMesh|SetStaticMesh (Variables|Default|GetStaticMesh) "/Game/UMG/Number_3D/Pachinko_number_7.Pachinko_number_7"))))