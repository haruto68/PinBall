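; BP_BlackHole is a pinball gimmick that pulls balls toward its center.
; An outer sphere overlap adds BP_Pinball actors to a target list, and leaving it removes them.
; Each Tick applies a mass-independent AddForce to each target's root component, directed at the black hole and scaled by ForcePower.
; Entering the inner center sphere also triggers target removal, intended to stop the pull at the core.
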(event OnComponentBeginOverlap(Sphere)
  (params (OverlappedComponent :type Primitive%20Component%20Object%20Reference) (OtherActor :type Actor%20Object%20Reference) (OtherComp :type Primitive%20Component%20Object%20Reference) (OtherBodyIndex :type Integer) (bFromSweep :type Boolean) (SweepResult :type Hit%20Result%20Structure%20%28by%20ref%29))
  ;[1 1 1] 吸い込む対象の配列追加＆削除
  (Utilities|Casting|CastToBP_Pinball OtherActor)
  (Utilities|Array|AddUnique (Variables|Default|GetTargetsToPull) OtherActor))

(event OnComponentEndOverlap(Sphere)
  (params (OverlappedComponent :type Primitive%20Component%20Object%20Reference) (OtherActor :type Actor%20Object%20Reference) (OtherComp :type Primitive%20Component%20Object%20Reference) (OtherBodyIndex :type Integer))
  ;[1 1 1] 吸い込む対象の配列追加＆削除
  (Utilities|Array|RemoveItem (Variables|Default|GetTargetsToPull) (stale OnComponentBeginOverlap(Sphere_center) OtherActor)))

(event OnComponentBeginOverlap(Sphere_center)
  (params (OverlappedComponent :type Primitive%20Component%20Object%20Reference) (OtherActor :type Actor%20Object%20Reference) (OtherComp :type Primitive%20Component%20Object%20Reference) (OtherBodyIndex :type Integer) (bFromSweep :type Boolean) (SweepResult :type Hit%20Result%20Structure%20%28by%20ref%29))
  ;[1 1 1] 吸い込む対象の配列追加＆削除
  (Utilities|Array|RemoveItem (Variables|Default|GetTargetsToPull) OtherActor))

(event EventTick
  (params (DeltaSeconds :type Float%20%28single-precision%29))
  ;[1 1 1] 吸い込み処理
  (for _array_element (Variables|Default|GetTargetsToPull)
    (bind _asprimitive_component (Utilities|Casting|CastToPrimitiveComponent (Variables|/Script/Engine.Actor|GetRootComponent _array_element)))
    (Physics|AddForce _asprimitive_component (* (Math|Vector|Normalize (- (Transformation|GetActorLocation) (Transformation|GetActorLocation _array_element))) (Variables|Default|GetForcePower)) "None" true)))

(event EventBeginPlay)

(fn ConstructionScript)