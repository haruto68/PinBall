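; Pinball stock indicator that shows the game mode's Stock count as a row of lamps built from InstancedStaticMesh instances on BeginPlay.
; Tick polls Stock; within the lamp count it applies M_Lamp and lights blue lamps through per-instance custom data.
; Above that count it switches to M_Illumination, writing staggered timing, wave interval, intensity and per-lamp colors as custom data.
; The tiered overflow coloring in MakeOver_Color is left unconnected.
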(event Custom|MakeColor_Lamp
  (params (index :type Integer))
  (bind (_r _g _b) (Math|Color|BreakColor "(R=0.000000,G=0.000000,B=255.000000,A=1.000000)"))
  ;[1 1 1] 色作成_ランプ
  (Variables|Default|SetIn%20Color (Utilities|Struct|MakeLinearColor _r _g _b 1.0)))

(event Custom|SetColor_Lamp
  (params (index :type Integer))
  (bind _instancedstaticmesh (Variables|Default|GetInstancedStaticMesh))
  (bind _in_color (Variables|Default|GetIn%20Color))
  (bind (_r _g _b) (Math|Color|BreakColor _in_color))
  ;[1 1 1] 色設定_ランプ
  (Components|InstancedStaticMesh|SetCustomDataValue _instancedstaticmesh index 1 _r true)
  (Components|InstancedStaticMesh|SetCustomDataValue _instancedstaticmesh index 2 _g true)
  (Components|InstancedStaticMesh|SetCustomDataValue _instancedstaticmesh index 3 _b true))

(event Custom|MakeColor_Illumination
  (params (index :type Integer))
  (bind (_r _g _b) (Math|Color|BreakColor "(R=255.000000,G=255.000000,B=0.000000,A=1.000000)"))
  (bind (_r_2 _g_2 _b_2) (Math|Color|BreakColor "(R=255.000000,G=0.000000,B=0.000000,A=1.000000)"))
  (bind (_r_3 _g_3 _b_3) (Math|Color|BreakColor "(R=0.000000,G=1.000000,B=0.000000,A=1.000000)"))
  (bind (_r_4 _g_4 _b_4) (Math|Color|BreakColor "(R=0.000000,G=0.000000,B=255.000000,A=1.000000)"))
  (bind (_r_5 _g_5 _b_5) (Math|Color|BreakColor "(R=255.000000,G=0.000000,B=255.000000,A=1.000000)"))
  ;[1 1 1] 色作成_イルミネーション
  (switch int index
    (:0
      (Variables|Default|SetIn%20Color (Utilities|Struct|MakeLinearColor _r_2 _g_2 _b_2 1.0)))
    (:1
      (Variables|Default|SetIn%20Color (Utilities|Struct|MakeLinearColor _r _g _b 1.0)))
    (:2
      (Variables|Default|SetIn%20Color (Utilities|Struct|MakeLinearColor _r_3 _g_3 _b_3 1.0)))
    (:3
      (Variables|Default|SetIn%20Color (Utilities|Struct|MakeLinearColor _r_4 _g_4 _b_4 1.0)))
    (:4
      (Variables|Default|SetIn%20Color (Utilities|Struct|MakeLinearColor _r_5 _g_5 _b_5 1.0)))))

(event Custom|Set_Illumination
  (bind _instancedstaticmesh (Variables|Default|GetInstancedStaticMesh))
  ;[1 1 1] ランプを点滅させる
  (for _index (range 0 (- (Variables|Default|GetLightNum) 1))
    (Rendering|Material|SetMaterial _instancedstaticmesh _index "/Game/Material_Pinball/M_Illumination.M_Illumination")
    (Components|InstancedStaticMesh|SetCustomDataValue _instancedstaticmesh _index 0 (* (Math|Conversions|ToFloat(Integer) _index) (Variables|Default|GetLamp%20Speed)) true) ; 点灯タイミングをずらす
    (Components|InstancedStaticMesh|SetCustomDataValue _instancedstaticmesh _index 1 3.0 true) ; ウェーブの間隔
    (Components|InstancedStaticMesh|SetCustomDataValue _instancedstaticmesh _index 2 3.0 true) ; 光の強さ
    (CallFunction|MakeColorIllumination _index)
    (CallFunction|SetColorIllumination _index)))

(event Custom|Set_Lamp
  (bind _instancedstaticmesh (Variables|Default|GetInstancedStaticMesh))
  ;[1 1 1] ランプを点灯させる
  (for _index (range 0 (- (Variables|Default|GetLightNum) 1))
    (Rendering|Material|SetMaterial _instancedstaticmesh _index "/Game/Material_Pinball/M_Lamp.M_Lamp")
    (Components|InstancedStaticMesh|SetCustomDataValue _instancedstaticmesh _index 0 0.0 true)
    (CallFunction|MakeColorLamp _index)
    (CallFunction|SetColorLamp _index)))

(event Custom|SetColor_Illumination
  (params (index :type Integer))
  (bind _instancedstaticmesh (Variables|Default|GetInstancedStaticMesh))
  (bind _in_color (Variables|Default|GetIn%20Color))
  (bind (_r _g _b) (Math|Color|BreakColor _in_color))
  ;[1 1 1] 色設定_イルミネーション
  (Components|InstancedStaticMesh|SetCustomDataValue _instancedstaticmesh index 3 _r true)
  (Components|InstancedStaticMesh|SetCustomDataValue _instancedstaticmesh index 4 _g true)
  (Components|InstancedStaticMesh|SetCustomDataValue _instancedstaticmesh index 5 _b true))

(event Custom|MakeOver_Color
  (bind (_r _g _b) (Math|Color|BreakColor "(R=255.000000,G=0.000000,B=0.000000,A=1.000000)"))
  (bind (_r_2 _g_2 _b_2) (Math|Color|BreakColor "(R=0.000000,G=0.000000,B=255.000000,A=1.000000)"))
  (bind (_r_3 _g_3 _b_3) (Math|Color|BreakColor "(R=0.000000,G=255.000000,B=0.000000,A=1.000000)"))
  ;[1 1 1] 0~5 / 6~10 / 11~15 でランプの色を設定する
  (switch int (/ (Variables|Default|GetNow_Stock) 5)
    (:0
      (for _index (range 0 (- (Math|Integer|%(Integer) (Variables|Default|GetNow_Stock) 5) 1))
        (Variables|Default|SetIn%20Color (Utilities|Struct|MakeLinearColor _r_2 _g_2 _b_2 1.0))))
    (:1
      (Utilities|FlowControl|Sequence
        (:then_0
          (for _index_2 (range 0 (- (Math|Integer|%(Integer) (Variables|Default|GetNow_Stock) 5) 1))
            (Variables|Default|SetIn%20Color (Utilities|Struct|MakeLinearColor _r_3 _g_3 _b_3 1.0))))
        (:then_1
          (for _index_3 (range (Math|Integer|%(Integer) (Variables|Default|GetNow_Stock) 5) (Variables|Default|GetLightNum))
            (Variables|Default|SetIn%20Color (Utilities|Struct|MakeLinearColor _r_2 _g_2 _b_2 1.0))))))
    (:2
      (Utilities|FlowControl|Sequence
        (:then_0
          (for _index_4 (range 0 (- (Math|Integer|%(Integer) (Variables|Default|GetNow_Stock) 5) 1))
            (Variables|Default|SetIn%20Color (Utilities|Struct|MakeLinearColor _r _g _b 1.0))))
        (:then_1
          (for _index_5 (range (Math|Integer|%(Integer) (Variables|Default|GetNow_Stock) 5) (Variables|Default|GetLightNum))
            (Variables|Default|SetIn%20Color (Utilities|Struct|MakeLinearColor _r_3 _g_3 _b_3 1.0))))))))

(event EventBeginPlay
  (Utilities|FlowControl|Sequence
    (:then_0
      (for _index (range 0 (- (Variables|Default|GetLightNum) 1))
        ;[1 1 1] インスタンス作成
        (bind _returnvalue (Components|InstancedStaticMesh|AddInstance (Variables|Default|GetInstancedStaticMesh) (Math|Transform|MakeTransform (Math|Vector|MakeVector 0.0 (Math|Conversions|ToFloat(Integer) (* _index 200)) 0.0)) false))
        (CallFunction|MakeColorLamp _returnvalue)
        (CallFunction|SetColorLamp _returnvalue)))))

(event EventTick
  (params (DeltaSeconds :type Float%20%28single-precision%29))
  ;[1 1 1] ストック数に変化があった場合
  (bind _asbp_first_person_game_mode (Utilities|Casting|CastToBP_FirstPersonGameMode (Game|GetGameMode)))
  (bind _output_get (Variables|Default|SetNow_Stock (Variables|/Game/FirstPerson/Blueprints/BP_FirstPersonGameMode.BP_FirstPersonGameMode_C|GetStock _asbp_first_person_game_mode)))
  (if (!= _output_get (Variables|Default|GetOld_Stock))
    ;[1 1 1] ストック数がランプ数より大きいか
    (if (> (Variables|Default|GetNow_Stock) (Variables|Default|GetLightNum))
      (CallFunction|SetIllumination)
      (else
        (CallFunction|SetLamp)
        (Utilities|FlowControl|Sequence
          (:then_0
            ;[1 1 1] ストック数未満の引数を点灯
            (for _index (range 0 (- (Variables|Default|GetNow_Stock) 0))
              (Components|InstancedStaticMesh|SetCustomDataValue (Variables|Default|GetInstancedStaticMesh) _index 0 1.0 true)))
          (:then_1
            ;[1 1 1] ストック数以上の引数を消灯
            (for _index_2 (range (Variables|Default|GetNow_Stock) (Variables|Default|GetLightNum))
              (Components|InstancedStaticMesh|SetCustomDataValue (Variables|Default|GetInstancedStaticMesh) _index_2 0 0.0 true)))
          (:then_2
            (Variables|Default|SetOld_Stock (Variables|Default|GetNow_Stock))))))))

(fn ConstructionScript)