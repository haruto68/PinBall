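; BP_WaveLight builds a column of rainbow-colored wave lamps for the pinball game.
; On BeginPlay it adds instances to one InstancedStaticMesh, stepping down local Z.
; Per-instance custom data carries a staggered timing offset scaled by LampSpeed, wave interval, intensity and RGB color, presumably for the material to animate.
; Rainbow picks each color by index modulo 6, so its seventh case (magenta) never runs.
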(event Custom|Rainbow
  (params (index :type Integer))
  (bind (_r _g _b) (Math|Color|BreakColor "(R=255.000000,G=0.000000,B=255.000000,A=1.000000)"))
  (bind (_r_2 _g_2 _b_2) (Math|Color|BreakColor "(R=1.000000,G=0.350000,B=0.000000,A=1.000000)"))
  (bind (_r_3 _g_3 _b_3) (Math|Color|BreakColor "(R=255.000000,G=255.000000,B=0.000000,A=1.000000)"))
  (bind (_r_4 _g_4 _b_4) (Math|Color|BreakColor "(R=0.000000,G=255.000000,B=255.000000,A=1.000000)"))
  (bind (_r_5 _g_5 _b_5) (Math|Color|BreakColor "(R=255.000000,G=0.000000,B=0.000000,A=1.000000)"))
  (bind (_r_6 _g_6 _b_6) (Math|Color|BreakColor "(R=0.000000,G=0.000000,B=255.000000,A=1.000000)"))
  (bind (_r_7 _g_7 _b_7) (Math|Color|BreakColor "(R=0.000000,G=255.000000,B=0.000000,A=1.000000)"))
  (switch int (Math|Integer|%(Integer) index 6)
    (:0
      ;[1 1 1] 虹色
      (Variables|Default|SetIn%20Color (Utilities|Struct|MakeLinearColor _r_5 _g_5 _b_5 1.0)))
    (:1
      (Variables|Default|SetIn%20Color (Utilities|Struct|MakeLinearColor _r_2 _g_2 _b_2 1.0)))
    (:2
      (Variables|Default|SetIn%20Color (Utilities|Struct|MakeLinearColor _r_3 _g_3 _b_3 1.0)))
    (:3
      (Variables|Default|SetIn%20Color (Utilities|Struct|MakeLinearColor _r_7 _g_7 _b_7 1.0)))
    (:4
      (Variables|Default|SetIn%20Color (Utilities|Struct|MakeLinearColor _r_4 _g_4 _b_4 1.0)))
    (:5
      (Variables|Default|SetIn%20Color (Utilities|Struct|MakeLinearColor _r_6 _g_6 _b_6 1.0)))
    (:6
      (Variables|Default|SetIn%20Color (Utilities|Struct|MakeLinearColor _r _g _b 1.0)))))

(event EventBeginPlay
  (bind _instancedstaticmesh (Variables|Default|GetInstancedStaticMesh))
  (bind _instancedstaticmesh_2 (Variables|Default|GetInstancedStaticMesh))
  (bind _in_color (Variables|Default|GetIn%20Color))
  (bind (_r _g _b) (Math|Color|BreakColor _in_color))
  (for _index (range 0 (Variables|Default|GetLightNum))
    ;[1 1 1] インスタンス作成
    (bind _returnvalue (Components|InstancedStaticMesh|AddInstance (Variables|Default|GetInstancedStaticMesh) (Math|Transform|MakeTransform (Math|Vector|MakeVector 0.0 0.0 (Math|Conversions|ToFloat(Integer) (* _index -200)))) false))
    ;[1 1 1] インスタンスごとに光を設定
    (Components|InstancedStaticMesh|SetCustomDataValue _instancedstaticmesh_2 _returnvalue 0 (* (Math|Conversions|ToFloat(Integer) _returnvalue) (Variables|Default|Getlamp_speed)) true) ; 点灯タイミングをずらす
    (Components|InstancedStaticMesh|SetCustomDataValue _instancedstaticmesh_2 _returnvalue 1 1.0 true) ; ウェーブの間隔
    (Components|InstancedStaticMesh|SetCustomDataValue _instancedstaticmesh_2 _returnvalue 2 2.0 true) ; 光の強さ
    (CallFunction|Rainbow _returnvalue) ; 虹色に変色
    ;[1 1 1] 色設定
    (Components|InstancedStaticMesh|SetCustomDataValue _instancedstaticmesh _returnvalue 3 _r true)
    (Components|InstancedStaticMesh|SetCustomDataValue _instancedstaticmesh _returnvalue 4 _g true)
    (Components|InstancedStaticMesh|SetCustomDataValue _instancedstaticmesh _returnvalue 5 _b true)))

(fn ConstructionScript)