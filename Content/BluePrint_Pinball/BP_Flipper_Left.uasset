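; BP_Flipper_Left is the left pinball flipper, driven by physics and the IA_Left_Trigger Enhanced Input action, with player 0 input enabled on BeginPlay.
; While triggered, a velocity-change radial impulse from the Scene component's location pushes the flipper mesh.
; The PhysicsConstraint switches to SLERP angular drive on press, then back to Twist and Swing on release or cancel, which also plays a sound.
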(event Input|EnhancedActionEvents|EnhancedInputActionIA_Left_Trigger
  (params (ActionValue :type Boolean) (ElapsedSeconds :type Float%20%28double-precision%29) (TriggeredSeconds :type Float%20%28double-precision%29) (InputAction :type Input%20Action%20Object%20Reference :default "/Game/System_Pinball/Input/IA_Left_Trigger.IA_Left_Trigger"))
  (bind _physicsconstraint (Variables|Default|GetPhysicsConstraint))
  (:Triggered
    (Physics|AddRadialImpulse (Variables|Default|GetStaticMesh) (Transformation|GetWorldLocation (Variables|Default|GetScene)) 5e+02 4e+03 "RIF_Constant" true))
  (:Started
    (Class|PhysicsConstraintComponent|SetAngularDriveMode _physicsconstraint "SLERP"))
  (:Canceled
    (Class|PhysicsConstraintComponent|SetAngularDriveMode _physicsconstraint "TwistAndSwing" :!label _label)
    (Audio|PlaySound2D "/Game/Sound_PinBall/audiostock_728811.audiostock_728811" 1.0 1.0 0.0 0 0))
  (:Completed
    (goto _label)))

(event EventBeginPlay
  (Input|EnableInput (Game|GetPlayerController 0)))

(fn ConstructionScript)