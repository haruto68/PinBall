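; BP_Propeller is a pinball propeller that awards score based on the world pitch of its mesh.
; BeginPlay stores the actor's starting pitch once.
; Each Tick subtracts it from the absolute mesh pitch and, while the result is below a negative near-right-angle threshold, sends AddScore to BP_FirstPersonGameMode.
; The check has no latch, so score repeats every frame the condition holds.
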(event EventBeginPlay
  (Variables|Default|SetPrev%20Rotation (.pitch (Transformation|GetActorRotation))))

(event EventTick
  (params (DeltaSeconds :type Float%20%28single-precision%29))
  (if (< (- (Math|Float|Absolute(Float) (.pitch (Transformation|GetWorldRotation (Variables|Default|GetStaticMesh)))) (Variables|Default|GetPrev%20Rotation)) -89.0)
    (bind _asbp_first_person_game_mode (Utilities|Casting|CastToBP_FirstPersonGameMode (Game|GetGameMode)))
    (Default|EventAddScore _asbp_first_person_game_mode (Variables|Default|GetAddScore))))

(fn ConstructionScript)