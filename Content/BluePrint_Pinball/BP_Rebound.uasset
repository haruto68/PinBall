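; BP_Rebound is a pinball bumper that moves and rotates back and forth and knocks the ball away on contact.
; A timeline lerps the mesh from its start transform by EndLocation and EndRotation offsets, ping-ponging via a FlipFlop on Finished.
; On hitting a BP_Pinball, it applies an impulse along the negated hit normal scaled by ReboundPower, notifies BP_FirstPersonGameMode through HitRebound, and plays a provisional camera shake.
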(event EventBeginPlay
  ;[1 1 1] 往復移動＆回転ループ
  (Variables|Default|SetStartLocation (Transformation|GetWorldLocation (Variables|Default|GetStaticMesh)))
  (Variables|Default|SetStartRotation (Transformation|GetWorldRotation (Variables|Default|GetStaticMesh)))
  (bind _alpha (Timeline|TImeLine Play)
    (:Update
      (Transformation|SetWorldLocationAndRotation (Variables|Default|GetStaticMesh) (Math|Vector|Lerp(Vector) (Variables|Default|GetStartLocation) (+ (Variables|Default|GetStartLocation) (Variables|Default|GetEndLocation)) _alpha) (Math|Rotator|Lerp(Rotator) (Variables|Default|GetStartRotation) (Math|Rotator|CombineRotators (Variables|Default|GetStartRotation) (Variables|Default|GetEndRotation)) _alpha true) false false))
    (:Finished
      (Utilities|FlowControl|FlipFlop
        (:A
          (Timeline|TImeLine Reverse))
        (:B
          (Timeline|TImeLine Play))))))

(event Collision|EventHit
  (params (MyComp :type Primitive%20Component%20Object%20Reference) (Other :type Actor%20Object%20Reference) (OtherComp :type Primitive%20Component%20Object%20Reference) (bSelfMoved :type Boolean) (HitLocation :type Vector :default "0, 0, 0") (HitNormal :type Vector :default "0, 0, 0") (NormalImpulse :type Vector :default "0, 0, 0") (Hit :type Hit%20Result%20Structure%20%28by%20ref%29))
  (Utilities|Casting|CastToBP_Pinball Other)
  (Physics|AddImpulseatLocation OtherComp (* HitNormal (* (Variables|Default|GetRebound_Power) -1e+05)) HitLocation "None")
  (bind _asbp_first_person_game_mode (Utilities|Casting|CastToBP_FirstPersonGameMode (Game|GetGameMode)))
  (Default|HitRebound _asbp_first_person_game_mode)
  ;[1 1 1] カメラを揺らす（仮） 設定はCS_Base
  (Game|Feedback|ClientStartCameraShake (Game|GetPlayerController 0) "/Game/CameraShake/CS_Base.CS_Base_C" 1.0 "CameraLocal" "0, 0, 0"))

(fn ConstructionScript)