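; Pinball target with a row of lamps that knocks BP_Pinball away on hit and awards score.
; BeginPlay spawns the lamps as instanced static meshes, coloured through per-instance custom data.
; Each hit lights another lamp and sends AddScore to BP_FirstPersonGameMode; the final hit sends AddScore2 instead and calls Reset.
; Reset swaps to M_Illumination for blinking, then after a delay clears the count and restores M_Lamp unlit.
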(event Custom|SetColor
  (params (index :type Integer))
  (bind (_r _g _b) (Math|Color|BreakColor "(R=255.000000,G=0.000000,B=0.000000,A=1.000000)"))
  (bind (_r_2 _g_2 _b_2) (Math|Color|BreakColor "(R=0.000000,G=0.000000,B=255.000000,A=1.000000)"))
  (bind (_r_3 _g_3 _b_3) (Math|Color|BreakColor "(R=0.000000,G=255.000000,B=0.000000,A=1.000000)"))
  (switch int index
    (:0
      (Variables|Default|SetIn%20Color (Utilities|Struct|MakeLinearColor _r _g _b 1.0)))
    (:1
      (Variables|Default|SetIn%20Color (Utilities|Struct|MakeLinearColor _r_3 _g_3 _b_3 1.0)))
    (:2
      (Variables|Default|SetIn%20Color (Utilities|Struct|MakeLinearColor _r_2 _g_2 _b_2 1.0)))))

(event Custom|Reset
  (bind (_r _g _b) (Math|Color|BreakColor "(R=255.000000,G=0.000000,B=255.000000,A=1.000000)"))
  (bind _instancedstaticmesh (Variables|Default|GetInstancedStaticMesh))
  (bind _instancedstaticmesh_2 (Variables|Default|GetInstancedStaticMesh))
  (bind _instancedstaticmesh_3 (Variables|Default|GetInstancedStaticMesh))
  ;[1 1 1] ランプを点滅させる
  (for _index (range 0 (- (Variables|Default|GetLightNum) 1))
    (Rendering|Material|SetMaterial _instancedstaticmesh _index "/Game/Material_Pinball/M_Illumination.M_Illumination")
    (Components|InstancedStaticMesh|SetCustomDataValue _instancedstaticmesh _index 1 2.0 true)
    (Components|InstancedStaticMesh|SetCustomDataValue _instancedstaticmesh _index 2 0.1 true)
    (Components|InstancedStaticMesh|SetCustomDataValue _instancedstaticmesh_2 _index 3 _r true)
    (Components|InstancedStaticMesh|SetCustomDataValue _instancedstaticmesh_2 _index 4 _g true)
    (Components|InstancedStaticMesh|SetCustomDataValue _instancedstaticmesh_2 _index 5 _b true)
    (Utilities|FlowControl|Delay 3.0)
    ;[1 1 1] リセット
    (Variables|Default|Sethit_count 0)
    (for _index_2 (range 0 (- (Variables|Default|GetLightNum) 1))
      (Rendering|Material|SetMaterial _instancedstaticmesh_3 _index_2 "/Game/Material_Pinball/M_Lamp.M_Lamp")
      (Components|InstancedStaticMesh|SetCustomDataValue _instancedstaticmesh_3 _index_2 0 0.0 true))))

(event Collision|EventHit
  (params (MyComp :type Primitive%20Component%20Object%20Reference) (Other :type Actor%20Object%20Reference) (OtherComp :type Primitive%20Component%20Object%20Reference) (bSelfMoved :type Boolean) (HitLocation :type Vector :default "0, 0, 0") (HitNormal :type Vector :default "0, 0, 0") (NormalImpulse :type Vector :default "0, 0, 0") (Hit :type Hit%20Result%20Structure%20%28by%20ref%29))
  (Utilities|FlowControl|Sequence
    (:then_0
      (Utilities|Casting|CastToBP_Pinball Other)
      (Physics|AddImpulseatLocation OtherComp (* HitNormal (* (Variables|Default|GetRebound_Power) -1e+05)) HitLocation "None"))
    (:then_1
      ;[1 1 1] ヒット
      (Utilities|Casting|CastToBP_Pinball Other)
      (if (< (Variables|Default|Gethit_count) (Variables|Default|GetLightNum))
        (bind _output_get (Variables|Default|Sethit_count (+ (Variables|Default|Gethit_count) 1)))
        ;[1 1 1] ヒット数ごとに点灯
        (for _index (range 0 (- _output_get 1))
          (Components|InstancedStaticMesh|SetCustomDataValue (Variables|Default|GetInstancedStaticMesh) _index 0 1.0 true))
        ;[1 1 1] 全て点灯したらリセット
        (if (>= (Variables|Default|Gethit_count) (Variables|Default|GetLightNum))
          (CallFunction|Reset)
          (bind _asbp_first_person_game_mode (Utilities|Casting|CastToBP_FirstPersonGameMode (Game|GetGameMode)))
          (Default|EventAddScore _asbp_first_person_game_mode (Variables|Default|GetAddScore2))
          (else
            (bind _asbp_first_person_game_mode_2 (Utilities|Casting|CastToBP_FirstPersonGameMode (Game|GetGameMode)))
            (Default|EventAddScore _asbp_first_person_game_mode_2 (Variables|Default|GetAddScore))))))))

(event EventBeginPlay
  (bind _instancedstaticmesh (Variables|Default|GetInstancedStaticMesh))
  (bind _in_color (Variables|Default|GetIn%20Color))
  (bind (_r _g _b) (Math|Color|BreakColor _in_color))
  (for _index (range 0 (- (Variables|Default|GetLightNum) 1))
    ;[1 1 1] インスタンス作成
    (bind _returnvalue (Components|InstancedStaticMesh|AddInstance (Variables|Default|GetInstancedStaticMesh) (Math|Transform|MakeTransform (Math|Vector|MakeVector 0.0 (Math|Conversions|ToFloat(Integer) (* _index 200)) 0.0)) false))
    (CallFunction|SetColor _returnvalue)
    (Components|InstancedStaticMesh|SetCustomDataValue _instancedstaticmesh _returnvalue 1 _r true)
    (Components|InstancedStaticMesh|SetCustomDataValue _instancedstaticmesh _returnvalue 2 _g true)
    (Components|InstancedStaticMesh|SetCustomDataValue _instancedstaticmesh _returnvalue 3 _b true)))

(fn ConstructionScript)