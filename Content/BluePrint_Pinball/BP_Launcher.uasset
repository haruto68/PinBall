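; BP_Launcher is the pinball launcher that spawns and fires balls when the IA_Launcher input starts.
; It spawns a BP_Pinball at its Sphere through a SpawnActor gameplay task, then applies a mass-scaled, randomized impulse along the Arrow to pinballs overlapping the Sphere.
; Each launched ball passes a negative BallCost, chosen by level name on BeginPlay, to GMI_Pinball's SetScore.
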(event Custom|Launch
  ;[1 1 1] 発射
  (for _array_element (Collision|GetOverlappingActors (Variables|Default|GetSphere) "/Game/BluePrint_Pinball/BP_Pinball.BP_Pinball_C" :!class /Script/Engine.PrimitiveComponent)
    (bind _asprimitive_component (Utilities|Casting|CastToPrimitiveComponent (Variables|/Script/Engine.Actor|GetRootComponent _array_element)))
    (Physics|AddImpulse _asprimitive_component (* (Math|Vector|GetForwardVector (Variables|Default|GetArrow)) (* (Math|Random|RandomFloatinRange 0.8 1.2) (Variables|Default|GetLaunch_Power)) (Physics|GetMass _asprimitive_component)) "None" false)
    ;[1 1 1] スコアを1減らす
    (bind _asgmi_pinball (Utilities|Casting|CastToGMI_Pinball (Game|GetGameInstance)))
    (Default|SetScore _asgmi_pinball (Variables|Default|GetBallCost))))

(event Input|EnhancedActionEvents|EnhancedInputActionIA_Launcher
  (params (ActionValue :type Boolean) (ElapsedSeconds :type Float%20%28double-precision%29) (TriggeredSeconds :type Float%20%28double-precision%29) (InputAction :type Input%20Action%20Object%20Reference :default "/Game/System_Pinball/Input/IA_Launcher.IA_Launcher"))
  ;[1 1 1] 弾の生成と発射イベントの呼び出し
  (:Started
    (bind _returnvalue (AddComponent|AddGameplayTasksComponent))
    (|SpawnActor _returnvalue (Transformation|GetWorldLocation (Variables|Default|GetSphere)) "0, 0, 0" "/Game/BluePrint_Pinball/BP_Pinball.BP_Pinball_C" false 0
      (:then
        (CallFunction|Launch)))))

(event EventBeginPlay
  (Input|EnableInput (Game|GetPlayerController 0))
  (bind _returnvalue (Game|GetCurrentLevelName true))
  (if (Utilities|Enum|Equal(Enum) _returnvalue "Map_Level1")
    (Variables|Default|SetBallCost -1)
    (elif (Utilities|Enum|Equal(Enum) _returnvalue "Map_Level2")
      (Variables|Default|SetBallCost -100)
      (elif (Utilities|Enum|Equal(Enum) _returnvalue "Map_Level3")
        (Variables|Default|SetBallCost -5000)))))

(event Collision|EventActorBeginOverlap
  (params (OtherActor :type Actor%20Object%20Reference)))

(event EventTick
  (params (DeltaSeconds :type Float%20%28single-precision%29)))

(fn ConstructionScript)