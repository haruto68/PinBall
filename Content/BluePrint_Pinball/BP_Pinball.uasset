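; BP_Pinball is the ball actor of a pinball game, playing a shot sound when it spawns.
; Tick locks the physics Sphere to its starting X plane, applies a constant downward acceleration as pseudo-gravity, and spawns BP_GhostTrail afterimages at high speed.
; Hit ignores repeats of the last object and matches display names, destroying the ball shortly after certain boxes (drain or jammed launcher) and spawning sparks on BP_Rebound bumpers.
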(event EventBeginPlay
  ;[1 1 1] Wolrd Location のX座標を固定する
  (Variables|Default|SetStart%20Location%20X (.x (Transformation|GetWorldLocation (Variables|Default|GetSphere))))
  (Audio|PlaySound2D "/Game/Sound_PinBall/ショット.ショット" 1.0 1.0 0.0 0 0))

(event EventTick
  (params (DeltaSeconds :type Float%20%28single-precision%29))
  (bind _sphere (Variables|Default|GetSphere))
  (bind _returnvalue (Transformation|GetWorldLocation _sphere))
  ;[1 1 1] Wolrd Location のX座標を固定する
  (Transformation|SetWorldLocation _sphere (Math|Vector|MakeVector (Variables|Default|GetStart%20Location%20X) (.y _returnvalue) (.z _returnvalue)) false false)
  ;[1 1 1] 疑似的に重力量を設定する
  (Physics|AddForce (Variables|Default|GetSphere) "0.000000,0.000000,-1000.000000" "None" true)
  ;[1 1 1] 残像生成
  (if (> (Math|Vector|VectorLength (Transformation|GetVelocity)) 3e+03)
    (Game|SpawnActorfromClass "/Game/BluePrint_Pinball/BP_GhostTrail.BP_GhostTrail_C" (Transformation|GetActorTransform) "Undefined" 0 0)))

(event Collision|EventHit
  (params (MyComp :type Primitive%20Component%20Object%20Reference) (Other :type Actor%20Object%20Reference) (OtherComp :type Primitive%20Component%20Object%20Reference) (bSelfMoved :type Boolean) (HitLocation :type Vector :default "0, 0, 0") (HitNormal :type Vector :default "0, 0, 0") (NormalImpulse :type Vector :default "0, 0, 0") (Hit :type Hit%20Result%20Structure%20%28by%20ref%29))
  (bind _returnvalue (Utilities|GetDisplayName Other))
  ;[1 1 1] HitしたObjectを確認する
  (if (not (== Other (Variables|Default|GetHitObject_Name)))
    (bind _output_get (Variables|Default|SetHitObject_Name Other))
    ;[1 1 1] 「底面に触れる」または「発射口に詰まる」と自信を削除する
    (if (Math|Boolean|ORBoolean (Utilities|Enum|Equal(Enum) _returnvalue "Box3") (Utilities|Enum|Equal(Enum) _returnvalue "Box4") (Utilities|Enum|Equal(Enum) _returnvalue "Box5"))
      (Utilities|FlowControl|Delay 0.2)
      (Actor|DestroyActor)
      (else
        ;[1 1 1] BP_Reboundに触れたときパーティクルを生成
        (if (Utilities|String|Contains (Utilities|GetDisplayName _output_get) "BP_Rebound")
          (Niagara|SpawnSystematLocation "/Game/Niagara/NS_Spark.NS_Spark" (Transformation|GetWorldLocation (Variables|Default|GetSphere))))))))

(fn ConstructionScript)