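; BP_ScreenSaver is an actor whose static mesh bounces between walls in the Y-Z plane, like a screensaver.
; BeginPlay sets a diagonal velocity, which Tick adds to the mesh's world location every frame, unscaled by delta time.
; Plane overlaps with BP_Wall_LR flip Y velocity, and with BP_Wall_TB flip Z.
; A Timeline-driven back-and-forth Turn loop remains, but its only external call never runs.
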(event OnComponentBeginOverlap(Plane)
  (params (OverlappedComponent :type Primitive%20Component%20Object%20Reference) (OtherActor :type Actor%20Object%20Reference) (OtherComp :type Primitive%20Component%20Object%20Reference) (OtherBodyIndex :type Integer) (bFromSweep :type Boolean) (SweepResult :type Hit%20Result%20Structure%20%28by%20ref%29))
  (Utilities|Casting|CastToBP_Wall_LR OtherActor
    (:then
      (Variables|Default|SetVelocity (* (Variables|Default|GetVelocity) "0.000000,-1.000000,1.000000")))
    (:CastFailed
      (Utilities|Casting|CastToBP_Wall_TB OtherActor)
      (Variables|Default|SetVelocity (* (Variables|Default|GetVelocity) "0.000000,1.000000,-1.000000")))))

(event Custom|Turn
  (Development|PrintString "Start")
  ;[1 1 1] 往復移動＆回転ループ
  (Variables|Default|SetStartLocation (Transformation|GetWorldLocation (Variables|Default|GetStaticMesh)))
  (Variables|Default|SetStartRotation (Transformation|GetWorldRotation (Variables|Default|GetStaticMesh)))
  (Variables|Default|SetBreak%20Update false)
  (bind _alpha (Timeline|TImeLine PlayFromStart)
    (:Update
      (if (Variables|Default|GetBreak%20Update)
        (Timeline|TImeLine Stop)
        (elif true
          (Transformation|SetWorldLocationAndRotation (Variables|Default|GetStaticMesh) (Math|Vector|Lerp(Vector) (Variables|Default|GetStartLocation) (+ (Variables|Default|GetStartLocation) (Variables|Default|GetEndLocation)) _alpha) (Math|Rotator|Lerp(Rotator) (Variables|Default|GetStartRotation) (Math|Rotator|CombineRotators (Variables|Default|GetStartRotation) (Variables|Default|GetEndRotation)) _alpha true) false false))))
    (:Finished
      (Variables|Default|SetEndLocation (* (Variables|Default|GetEndLocation) "0.000000,-1.000000,0.000000"))
      (Development|PrintString "Finished")
      (CallFunction|Turn))))

(event EventBeginPlay
  (Variables|Default|SetVelocity "0.000000,10.000000,10.000000"))

(event EventTick
  (params (DeltaSeconds :type Float%20%28single-precision%29))
  (bind _staticmesh (Variables|Default|GetStaticMesh))
  (Transformation|SetWorldLocationAndRotation _staticmesh (+ (Transformation|GetWorldLocation _staticmesh) (Variables|Default|GetVelocity)) "0, 0, 0" false false))

(fn ConstructionScript)